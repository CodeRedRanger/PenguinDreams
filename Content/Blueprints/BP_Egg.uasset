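; BP_Egg is a physics egg that the player character bounces and that ends the game if it touches the landscape.
; Player overlap launches it with a fixed velocity, or triggers a squish loss if the player's IsGameOver flag is already set.
; Each loss branch runs once, halts player movement, prints an animation placeholder, waits, then opens the lose screen with UI-only input.
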(event `self.ReceiveBeginPlay`
  (bind _asbp_player_character (cast `/Game/Character/BP_PlayerCharacter` (`GameplayStatics.GetPlayerCharacter` 0)))
  (set `self.BP_PlayerCharacter` _asbp_player_character))

(event `self.EggCollision.OnComponentBeginOverlap`
  (params (OverlappedComponent :type "PrimitiveComponent Object Reference") (OtherActor :type "Actor Object Reference") (OtherComp :type "PrimitiveComponent Object Reference") (OtherBodyIndex :type Integer) (bFromSweep :type Boolean) (SweepResult :type "HitResult Structure (by ref)"))
  (bind _bp_playercharacter (`self.BP_PlayerCharacter`))
  (bind _bp_playercharacter_2 (`self.BP_PlayerCharacter`))
  (bind _bp_playercharacter_3 (`self.BP_PlayerCharacter`))
  (if (== OtherActor _bp_playercharacter)
    (if (and (`/Game/Character/BP_PlayerCharacter.IsGameOver` _bp_playercharacter) (`self.NotLost`))
      ;[1 1 1] Called so animation doesn't get called multiple times!
      (`/Engine/EditorBlueprintResources/StandardMacros.DoOnce` false
        (:`Completed`
          (set `/Game/Character/BP_PlayerCharacter.IsGameOver` true (`self.BP_PlayerCharacter`))
          (set `self.NotLost` false)
          ;[1 1 1] Stops being able to move
          (`self.DisableInput` _bp_playercharacter_2 (`GameplayStatics.GetPlayerController` 0))
          (`MovementComponent.StopMovementImmediately` (`Character.CharacterMovement` _bp_playercharacter_2))
          ;[1 1 1] Animation of squishing goes here!
          (`KismetSystemLibrary.PrintString` "Playing Squish Animation! (2 Second Delay)")
          (`KismetSystemLibrary.Delay` 2.0)
          (`self.LoseScreen`)))
      (else
        (`PrimitiveComponent.SetPhysicsLinearVelocity` (`self.Egg`) (500.0 0.0 600.0) false "None")))
    (elif (and (== (`GameplayStatics.GetObjectClass` OtherActor) "/Script/Landscape.LandscapeStreamingProxy") (`self.NotLost`))
      ;[1 1 1] Called so this doesn't get called multiple times!
      (`/Engine/EditorBlueprintResources/StandardMacros.DoOnce` false
        (:`Completed`
          (set `/Game/Character/BP_PlayerCharacter.IsGameOver` true (`self.BP_PlayerCharacter`))
          (set `self.NotLost` false)
          ;[1 1 1] Stops being able to move
          (`self.DisableInput` _bp_playercharacter_3 (`GameplayStatics.GetPlayerController` 0))
          (`MovementComponent.StopMovementImmediately` (`Character.CharacterMovement` _bp_playercharacter_3))
          ;[1 1 1] Animation of egg breaking goes here!
          (`KismetSystemLibrary.PrintString` "Playing Egg Cracking Animation! (2 Second Delay)")
          (`KismetSystemLibrary.Delay` 2.0)
          (`self.LoseScreen`))))))

(event `LoseScreen`
  (bind _returnvalue (`GameplayStatics.GetPlayerController` 0))
  ;[1 1 1] Creates Lose Screen Widget and Freezes Player Character from Moving
  (bind _returnvalue_2 (`|CreateWidget` "/Game/UI/WBP_LoseScreen.WBP_LoseScreen_C" _returnvalue))
  (`UserWidget.AddToViewport` _returnvalue_2 0)
  (`WidgetBlueprintLibrary.SetInputMode_UIOnlyEx` _returnvalue _returnvalue_2)
  (set `PlayerController.bShowMouseCursor` true (`GameplayStatics.GetPlayerController` 0)))

(fn `UserConstructionScript`)