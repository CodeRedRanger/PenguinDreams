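; BP_Camera is a follow camera actor that becomes the first player's view target on BeginPlay and snaps to the player character's location.
; Each tick it matches the character's X, offsets Y by CameraDistance and holds Z at CameraHeight, ignoring the character's vertical movement.
; Following pauses while the character's mesh simulates physics.
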(event `self.ReceiveBeginPlay`
  ;[1 1 1] On beginplay move camera to player and make character posses camera
  (`PlayerController.SetViewTargetWithBlend` (`GameplayStatics.GetPlayerController` 0) self 0.0 "VTBlend_Linear" 0.0 false)
  (`self.K2_SetActorLocation` (`self.K2_GetActorLocation` (`GameplayStatics.GetPlayerCharacter` 0))))

(event `self.ReceiveTick`
  (params (DeltaSeconds :type "Float (single-precision)"))
  (bind _returnvalue (`GameplayStatics.GetPlayerCharacter` 0))
  (bind (_returnvalue_x _returnvalue_y) (`KismetMathLibrary.BreakVector` (`self.K2_GetActorLocation` _returnvalue)))
  ;[1 1 1] On event tick move camera to player
  (if (not (`SceneComponent.IsSimulatingPhysics` (`Character.Mesh` _returnvalue) "None"))
    (`self.K2_SetActorLocation` (`KismetMathLibrary.MakeVector` _returnvalue_x (+ _returnvalue_y (`self.CameraDistance`)) (`self.CameraHeight`)))))

(fn `UserConstructionScript`)