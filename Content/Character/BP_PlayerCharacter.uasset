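; Player character that keeps moving forward along its control yaw, with move input slowing it or speeding it up, plus jump.
; BeginPlay adds the default Enhanced Input context, caches the BP_Camera actor and spawns a BP_Egg ahead of and above the capsule.
; Tick applies moderate forward input until IA_Move takes control, then the input's X sign picks a low or high scale.
; IA_Move also prints a debug string while triggered.
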(event `self.ReceiveBeginPlay`
  (bind _returnvalue (`SceneComponent.K2_GetComponentToWorld` (`self.CapsuleComponent`)))
  (bind _asplayer_controller (cast `PlayerController` (`self.GetController`)))
  (bind _returnvalue_2 (pcsubsystem `EnhancedInputLocalPlayerSubsystem` _asplayer_controller))
  (`/Engine/EditorBlueprintResources/StandardMacros.IsValid` _returnvalue_2
    (:`Is Valid`
      (`EnhancedInputSubsystemInterface.AddMappingContext` _returnvalue_2 "/Game/Character/Input/IMC_Default.IMC_Default" 0 (struct))
      (bind _returnvalue_3 (`GameplayStatics.GetActorOfClass` "/Game/Blueprints/BP_Camera.BP_Camera_C"))
      (set `self.BP_Camera` _returnvalue_3)
      (`|SpawnActorFromClass` "/Game/Blueprints/BP_Egg.BP_Egg_C" (`KismetMathLibrary.MakeTransform` (`KismetMathLibrary.MakeVector` (+ (.x (.location _returnvalue)) 40.0) (.y (.location _returnvalue)) (+ (.z (.location _returnvalue)) 120.0)) (.rotation _returnvalue) (.scale _returnvalue)) "Undefined" "MultiplyWithRoot" null null))))

(event `self.ReceiveTick`
  (params (DeltaSeconds :type "Float (single-precision)"))
  (bind (_returnvalue_roll _returnvalue_pitch _returnvalue_yaw) (`KismetMathLibrary.BreakRotator` (`self.GetControlRotation`)))
  (if (not (`self.IsInControl`))
    (`self.AddMovementInput` (`KismetMathLibrary.GetForwardVector` (`KismetMathLibrary.MakeRotator` 0.0 0.0 _returnvalue_yaw)) 0.5)))

(event `EnhancedInput|/Game/Character/Input/Actions/IA_Move`
  (params (ActionValue :type "Vector2D Structure") (ElapsedSeconds :type "Float (double-precision)") (TriggeredSeconds :type "Float (double-precision)") (InputAction :type "InputAction Object Reference" :default "/Game/Character/Input/Actions/IA_Move.IA_Move"))
  (bind (_returnvalue_roll _returnvalue_pitch _returnvalue_yaw) (`KismetMathLibrary.BreakRotator` (`self.GetControlRotation`)))
  (:`Triggered`
    (`KismetSystemLibrary.PrintString` "Hello")
    (`self.AddMovementInput` (`KismetMathLibrary.GetForwardVector` (`KismetMathLibrary.MakeRotator` 0.0 0.0 _returnvalue_yaw)) (select `bool` (< ActionValue_X 0.0) :`false` 2.0 :`true` 0.1)))
  (:`Started`
    (set `self.IsInControl` true))
  (:`Completed`
    (set `self.IsInControl` false)))

(event `EnhancedInput|/Game/Character/Input/Actions/IA_Jump`
  (params (ActionValue :type Boolean) (ElapsedSeconds :type "Float (double-precision)") (TriggeredSeconds :type "Float (double-precision)") (InputAction :type "InputAction Object Reference" :default "/Game/Character/Input/Actions/IA_Jump.IA_Jump"))
  (:`Triggered`
    (`self.Jump`)))

(fn `UserConstructionScript`)